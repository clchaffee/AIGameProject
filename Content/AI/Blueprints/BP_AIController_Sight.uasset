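; AI controller for a sight-based enemy in a horror game, running BT_Enemy on possess.
; Perception updates record a seen player in the Blackboard and flag the horror UI; otherwise a timer delays clearing line of sight and target.
; It also reacts to tagged creatures: a chasing Hearing creature becomes its alert target, while a Smell creature's position becomes its patrol location if LastKnownLocation is set.
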(event OnTargetPerceptionUpdated(AIPerception)
  (params (Actor :type Actor%20Object%20Reference) (Stimulus :type AI%20Stimulus%20Structure))
  (bind _blackboard (Variables|Default|GetBlackboard))
  (bind _blackboard_2 (Variables|Default|GetBlackboard))
  (bind _blackboard_3 (Variables|Default|GetBlackboard))
  (Utilities|FlowControl|Sequence
    (:then_0
      (if (and (Actor|ActorHasTag Actor "Player") (Utilities|Struct|BreakAIStimulus Stimulus))
        (Utilities|Time|ClearandInvalidateTimerbyHandle (Variables|Default|GetEnemyTimer))
        (AI|Components|Blackboard|SetValueasBool _blackboard (Variables|Default|GetHasLOS) true)
        (AI|Components|Blackboard|SetValueasObject _blackboard (Variables|Default|GetEnemyActor) Actor)
        (bind _asbp_horror_player_controller (Utilities|Casting|CastToBP_HorrorPlayerController (Game|GetPlayerController 0)))
        (Default|SetSight (Variables|/Game/Variant_Horror/Blueprints/BP_HorrorPlayerController.BP_HorrorPlayerController_C|GetHorror%20UI _asbp_horror_player_controller) true)
        (else
          (bind _returnvalue (Utilities|Time|SetTimerbyEvent (delegate Custom|StartEnemyTimer) (Variables|Default|GetLOSTimer)))
          (Variables|Default|SetEnemyTimer _returnvalue))))
    (:then_1
      ;[0.15 0.15 0.15 0.5] Checks to see if the actor it sees is the Hearing
      (if (and (Actor|ActorHasTag Actor "Hearing") (Utilities|Struct|BreakAIStimulus Stimulus))
        ;[0.15 0.15 0.15 0.5] Checks if the hearing creature is actively chasing (checks blackboard)
        (if (ScalableFloat|GetValueasBool (AI|GetBlackboard Actor) (Utilities|Name|MakeLiteralName "IsChasing"))
          ;[0.15 0.15 0.15 0.5] Success Condition
          (Development|PrintString "I have noted the hearing creature!")
          ;;[0.15 0.15 0.15 0.5] Sets IsAlerted to True, sets ChasingActor to Hearing Creature
          (AI|Components|Blackboard|SetValueasObject _blackboard_3 (Utilities|Name|MakeLiteralName "ChasingActor") Actor)
          (AI|Components|Blackboard|SetValueasBool _blackboard_3 (Utilities|Name|MakeLiteralName "IsAlerted") true)
          (else
            ;[0.15 0.15 0.15 0.5] Fail Condition
            (Development|PrintString "Hark! The creature was sighted yet it was not chasing anyone!")))))
    (:then_2
      (if (and (Actor|ActorHasTag Actor "Smell") (Utilities|Struct|BreakAIStimulus Stimulus))
        (if (Class|BlackboardComponent|IsVectorValueSet (Variables|Default|GetBlackboard) (Utilities|Name|MakeLiteralName "LastKnownLocation"))
          (AI|Components|Blackboard|SetValueasBool _blackboard_2 (Utilities|Name|MakeLiteralName "IsAlerted") true)
          (AI|Components|Blackboard|SetValueasVector _blackboard_2 (Utilities|Name|MakeLiteralName "PatrolLocation") (Transformation|GetActorLocation Actor)))))))

(event Custom|StartEnemyTimer
  (bind _blackboard (Variables|Default|GetBlackboard))
  (AI|Components|Blackboard|SetValueasBool _blackboard (Variables|Default|GetHasLOS) false)
  (AI|Components|Blackboard|SetValueasObject _blackboard (Variables|Default|GetEnemyActor) 0))

(event EventPossess
  (params (PossessedPawn :type Pawn%20Object%20Reference))
  (AI|RunBehaviorTree "/Game/AI/BehaviorTrees/BT_Enemy.BT_Enemy"))

(fn ConstructionScript)