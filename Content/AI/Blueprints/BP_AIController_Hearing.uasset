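; AI controller for a hearing-driven enemy that runs the BT_Enemy_Hearing behavior tree on possess.
; When AI perception hears an actor tagged Player, it writes the stimulus location to the LastHeardLocation blackboard key and switches on the sound indicator in the player controller's HorrorUI.
; A separate HandleHearSense function writes heard locations to a TargetLocation key, but nothing in this Blueprint calls it.
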(event OnTargetPerceptionUpdated(AIPerception)
  (params (Actor :type Actor%20Object%20Reference) (Stimulus :type AI%20Stimulus%20Structure))
  (bind (_age _expirationage _strength _stimuluslocation _receiverlocation _tag _bsuccessfullysensed) (Utilities|Struct|BreakAIStimulus Stimulus))
  (if (and (Actor|ActorHasTag Actor "Player") _bsuccessfullysensed)
    (bind _returnvalue (Class|AIPerceptionSystem|GetSenseClassforStimulus Stimulus))
    (if (== _returnvalue "/Script/AIModule.AISense_Hearing")
      (AI|Components|Blackboard|SetValueasVector (Variables|Default|GetBlackboard) (Utilities|Name|MakeLiteralName "LastHeardLocation") _stimuluslocation)
      (bind _asbp_horror_player_controller (Utilities|Casting|CastToBP_HorrorPlayerController (Game|GetPlayerController 0)))
      (Default|SetSound (Variables|/Game/Variant_Horror/Blueprints/BP_HorrorPlayerController.BP_HorrorPlayerController_C|GetHorror%20UI _asbp_horror_player_controller) true))))

(event EventPossess
  (params (PossessedPawn :type Pawn%20Object%20Reference))
  (AI|RunBehaviorTree "/Game/AI/BehaviorTrees/BT_Enemy_Hearing.BT_Enemy_Hearing"))

(fn ConstructionScript)

(fn HandleHearSense
  (params (Stimulus :type AI%20Stimulus%20Structure%20%28by%20ref%29))
  (bind _returnvalue (Class|AIPerceptionSystem|GetSenseClassforStimulus Stimulus))
  (if (== _returnvalue "/Script/AIModule.AISense_Hearing")
    (AI|Components|Blackboard|SetValueasVector (Variables|Default|GetBlackboard) (Variables|Default|GetTargetLocation) (.StimulusLocation (Utilities|Struct|BreakAIStimulus Stimulus)))))