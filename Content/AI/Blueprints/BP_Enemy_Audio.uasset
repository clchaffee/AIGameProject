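; BP_Enemy_Audio is an enemy Blueprint that ends the game when it touches the horror character.
; A capsule hit on BP_HorrorCharacter makes the player controller's HorrorUI show the lose screen, naming "Smell Creature" as the killer despite the asset's Audio name.
; It then disables player input and stops the game mode's timer.
; The construction script only calls its parent.
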(event OnComponentHit(CapsuleComponent)
  (params (HitComponent :type Primitive%20Component%20Object%20Reference) (OtherActor :type Actor%20Object%20Reference) (OtherComp :type Primitive%20Component%20Object%20Reference) (NormalImpulse :type Vector :default "0, 0, 0") (Hit :type Hit%20Result%20Structure%20%28by%20ref%29))
  (Utilities|Casting|CastToBP_HorrorCharacter OtherActor)
  (bind _asbp_horror_player_controller (Utilities|Casting|CastToBP_HorrorPlayerController (Game|GetPlayerController 0)))
  (Default|UpdateKilledInfoDesc (Variables|/Game/Variant_Horror/Blueprints/BP_HorrorPlayerController.BP_HorrorPlayerController_C|GetHorror%20UI _asbp_horror_player_controller) (Utilities|Text|MakeLiteralText "Smell Creature"))
  (Widget|SetVisibility (Variables|/Game/Variant_Horror/UI/UI_Horror.UI_Horror_C|GetLoseScreen (Variables|/Game/Variant_Horror/Blueprints/BP_HorrorPlayerController.BP_HorrorPlayerController_C|GetHorror%20UI _asbp_horror_player_controller)) "Visible")
  (Default|DisablePlayerInput _asbp_horror_player_controller)
  (bind _asbp_horror_game_mode (Utilities|Casting|CastToBP_HorrorGameMode (Game|GetGameMode)))
  (Default|StopTimerEvent _asbp_horror_game_mode))

(fn ConstructionScript
  (|CallParentFunction))