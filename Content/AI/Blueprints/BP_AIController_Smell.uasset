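; AI controller for the smell-based enemy, which chases the horror character when it releases pheromone.
; On possess it runs the smell behavior tree, and on BeginPlay it caches the controlled enemy and player character.
; Perception updates for a Player-tagged actor during pheromone release set the enemy chasing and write the player's location to the blackboard.
; Other updates only print debug values; pheromone-reset logic is left unconnected.
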(event OnTargetPerceptionUpdated(AIPerception)
  (params (Actor :type Actor%20Object%20Reference) (Stimulus :type AI%20Stimulus%20Structure))
  (bind _returnvalue (Actor|ActorHasTag Actor "Player"))
  (bind _bp_horror_character_ref (Variables|Default|GetBP%20Horror%20Character%20Ref))
  (bind _releasepheromone (Variables|/Game/Variant_Horror/Blueprints/BP_HorrorCharacter.BP_HorrorCharacter_C|GetReleasePheromone _bp_horror_character_ref))
  (if (and _releasepheromone _returnvalue)
    (Development|PrintString "chase player" true true "(R=0.000000,G=1.000000,B=0.010659,A=1.000000)" 3.0)
    (Variables|/Game/AI/Blueprints/BP_Enemy_Smell.BP_Enemy_Smell_C|SetIsChasing? (Variables|Default|GetBP%20Enemy%20Smell%20Ref) true)
    (AI|Components|Blackboard|SetValueasVector (Variables|Default|GetBlackboard) (Variables|Default|GetLastKnownLocation) (Transformation|GetActorLocation (Variables|Default|GetBP%20Horror%20Character%20Ref)))
    (else
      (Development|PrintString (Utilities|String|Append "1st: " (Utilities|String|ToString(Boolean) _releasepheromone) " 2nd: " (Utilities|String|ToString(Boolean) _returnvalue) " 3rd: " (Utilities|String|ToString(Boolean) (.bSuccessfullySensed (Utilities|Struct|BreakAIStimulus Stimulus)))) true true "(R=1.000000,G=0.000000,B=0.685096,A=1.000000)" 4.0))))

(event EventBeginPlay
  (Utilities|FlowControl|Sequence
    (:then_0
      (bind _asbp_enemy_smell (Utilities|Casting|CastToBP_Enemy_Smell (Pawn|GetControlledPawn self))
        (:then
          (Variables|Default|SetBP%20Enemy%20Smell%20Ref _asbp_enemy_smell))
        (:CastFailed
          (Development|PrintString "cast failed: smell ai"))))
    (:then_1
      (bind _asbp_horror_character (Utilities|Casting|CastToBP_HorrorCharacter (Game|GetPlayerCharacter 0))
        (:then
          (Variables|Default|SetBP%20Horror%20Character%20Ref _asbp_horror_character))
        (:CastFailed
          (Development|PrintString "cast failed: horror character"))))))

(event EventPossess
  (params (PossessedPawn :type Pawn%20Object%20Reference))
  (AI|RunBehaviorTree "/Game/AI/BehaviorTrees/BT_Enemy_Smell.BT_Enemy_Smell"))

(event EventTick
  (params (DeltaSeconds :type Float%20%28single-precision%29)))

(fn ConstructionScript)