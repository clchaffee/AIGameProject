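; Test enemy AI controller that runs the BT_EnemyTesting behavior tree on possess and handles spotting the player.
; Perception updates set HasLOS and EnemyActor on the blackboard when a Player-tagged actor is sensed, and turn on the horror UI's sight indicator.
; Other updates start a LOSTimer delay that clears both keys, without resetting the indicator.
; Smell and hearing alert branches exist but are disconnected.
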(event OnTargetPerceptionUpdated(AIPerception)
  (params (Actor :type Actor%20Object%20Reference) (Stimulus :type AI%20Stimulus%20Structure))
  (bind _blackboard (Variables|Default|GetBlackboard))
  (Utilities|FlowControl|Sequence
    (:then_0
      (if (and (Actor|ActorHasTag Actor "Player") (Utilities|Struct|BreakAIStimulus Stimulus))
        (Utilities|Time|ClearandInvalidateTimerbyHandle (Variables|Default|GetEnemyTimer))
        (AI|Components|Blackboard|SetValueasBool _blackboard (Variables|Default|GetHasLOS) true)
        (AI|Components|Blackboard|SetValueasObject _blackboard (Variables|Default|GetEnemyActor) Actor)
        (bind _asbp_horror_player_controller (Utilities|Casting|CastToBP_HorrorPlayerController (Game|GetPlayerController 0)))
        (Default|SetSight (Variables|/Game/Variant_Horror/Blueprints/BP_HorrorPlayerController.BP_HorrorPlayerController_C|GetHorror%20UI _asbp_horror_player_controller) true)
        (else
          (bind _returnvalue (Utilities|Time|SetTimerbyEvent (delegate Custom|StartEnemyTimer) (Variables|Default|GetLOSTimer)))
          (Variables|Default|SetEnemyTimer _returnvalue))))
    (:then_3
      (Development|PrintString "Hello"))))

(event Custom|StartEnemyTimer
  (bind _blackboard (Variables|Default|GetBlackboard))
  (AI|Components|Blackboard|SetValueasBool _blackboard (Variables|Default|GetHasLOS) false)
  (AI|Components|Blackboard|SetValueasObject _blackboard (Variables|Default|GetEnemyActor) 0))

(event EventPossess
  (params (PossessedPawn :type Pawn%20Object%20Reference))
  (AI|RunBehaviorTree "/Game/AI/TEST_AIINTERACTION/BT_EnemyTesting.BT_EnemyTesting"))

(fn ConstructionScript)